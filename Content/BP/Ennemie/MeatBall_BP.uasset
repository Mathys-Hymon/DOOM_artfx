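; MeatBall_BP is an enemy that fires homing Ennemie_Bullet projectiles at the player it has seen.
; Shoot is gated by a DoOnce, switches State and holds Hit true for half the flipbook's length while spawning a bullet just ahead of the actor.
; SpawnBulletSRV creates the bullet, then SpawnBulletMC sets its homing target from PlayerSeen and re-arms shooting after a fixed cooldown.
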(event `self.Shoot`
  (`/Engine/EditorBlueprintResources/StandardMacros.DoOnce` false :!label _label
    (:`Completed`
      (`|ExecutionSequence`
        (:`then_0`
          (set `self.state` 2)
          (set `self.hit` true)
          (`KismetSystemLibrary.Delay` (/ (`PaperFlipbookComponent.GetFlipbookLength` (`self.PaperFlipbook`)) 2.0))
          (set `self.hit` false))
        (:`then_1`
          (`self.SpawnBulletSRV` (`KismetMathLibrary.Conv_VectorToTransform` (+ (`self.K2_GetActorLocation`) (* (`self.GetActorForwardVector`) 20.0)))))))))

(event `ResetShoot`
  (goto _label :!via `Reset`))

(event `SpawnBulletSRV`
  (params (SpawnTransform :type "Transform Structure"))
  (bind _returnvalue (`|SpawnActorFromClass` "/Game/BP/Ennemie/Ennemie_Bullet.Ennemie_Bullet_C" SpawnTransform "AlwaysSpawn" "MultiplyWithRoot" null null))
  (`self.SpawnBulletMC` _returnvalue))

(event `SpawnBulletMC`
  (params (Target :type "/Game/BP/Ennemie/Ennemie_Bullet Object Reference"))
  (set `ProjectileMovementComponent.HomingTargetComponent` (`/Game/BP/Player/BP_Player.Scene` (`self.PlayerSeen`)) (`/Game/BP/Ennemie/Ennemie_Bullet.ProjectileMovement` Target))
  (`KismetSystemLibrary.Delay` 3.0)
  (`self.ResetShoot`))

(fn `UserConstructionScript`
  (`parent.UserConstructionScript`))