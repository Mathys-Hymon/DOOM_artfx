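; Zombie enemy Blueprint that implements its attack on top of a parent class.
; ShootMC, gated by a DoOnce, sets the attack state and Hit flag, captures a point just behind the seen player, then line traces to it after a brief delay.
; Any valid hit actor receives damage through GetHitMessage.
; After half the flipbook's length, Hit clears and ResetShoot reopens the gate.
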(event `self.ShootMC`
  (bind _playerseen (`self.PlayerSeen`))
  (`/Engine/EditorBlueprintResources/StandardMacros.DoOnce` false :!label _label
    (:`Completed`
      (`|ExecutionSequence`
        (:`then_0`
          (set `self.state` 2)
          (set `self.hit` true)
          (bind _output_get (set `self.LastLocation` (- (`self.K2_GetActorLocation` _playerseen) (* (`self.GetActorForwardVector` _playerseen) 3))))
          (`KismetSystemLibrary.Delay` 0.1)
          (bind _outhit (`KismetSystemLibrary.LineTraceSingle` (`self.K2_GetActorLocation`) _output_get "TraceTypeQuery2"))
          (bind (_bblockinghit _binitialoverlap _time _distance _location _impactpoint _normal _impactnormal _physmat _hitactor) (`GameplayStatics.BreakHitResult` _outhit))
          (`/Engine/EditorBlueprintResources/StandardMacros.IsValid` _hitactor
            (:`Is Valid`
              (message `/Game/BP/Player/BPI_Player.GetHit` _hitactor (`self.Damages`)))
            (:`Is Not Valid`
              _))
          (`KismetSystemLibrary.Delay` (/ (`PaperFlipbookComponent.GetFlipbookLength` (`self.PaperFlipbook`)) 2.0))
          (set `self.hit` false)
          (`self.ResetShoot`))))))

(event `ResetShoot`
  (goto _label :!via `Reset`))

(fn `UserConstructionScript`
  (`parent.UserConstructionScript`))