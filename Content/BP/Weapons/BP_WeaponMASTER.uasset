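; Master weapon actor serving as both a player-facing floor pickup that passes its data to the inventory and a flipbook-animated weapon.
; Manual weapons fire once per shot animation through a DoOnce, while automatic ones fire on each ShootLoop call, dividing damage by DeltaSeconds.
; FireWeapon sweeps a vertical stack of line traces, reporting the first enemy hit to the player, or a parry for punches hitting mid-close non-enemy actors.
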(event `/Game/BP/Weapons/BPI_Weapon.SetSpriteVisible`
  (params (visible :type Boolean))
  (`SceneComponent.SetVisibility` (`self.FloorSprite`) visible false)
  (`ActorComponent.K2_DestroyComponent` (`self.Sphere`)))

(event `GetData`
  (params (PC :type "/Game/BP/Player/BP_Player Object Reference"))
  (message `/Game/BP/Player/BPI_Player.AddToInventory` PC (make `/Game/BP/Weapons/WeaponData` (`self.ManualWeapon`) (`self.DistanceAttack`) (`self.weaponDamage`) (`self.Weapon Sprite`) (`self.Weapon Idle Anim`) (`self.Weapon Shoot Anim`) (`self.IsPunch`))))

(event `self.ReceiveTick`
  (params (DeltaSeconds :type "Float (single-precision)"))
  (bind (_returnvalue_roll _returnvalue_pitch _returnvalue_yaw) (`KismetMathLibrary.BreakRotator` (`KismetMathLibrary.FindLookAtRotation` (`self.K2_GetActorLocation`) (`self.K2_GetActorLocation` (`GameplayStatics.GetPlayerCharacter` 0)))))
  (set `self.Delta Seconds` DeltaSeconds)
  (if (`SceneComponent.bVisible` (`self.FloorSprite`))
    (`self.K2_SetActorRotation` (`KismetMathLibrary.MakeRotator` 0.0 0.0 _returnvalue_yaw))))

(event `self.Sphere.OnComponentBeginOverlap`
  (params (OverlappedComponent :type "PrimitiveComponent Object Reference") (OtherActor :type "Actor Object Reference") (OtherComp :type "PrimitiveComponent Object Reference") (OtherBodyIndex :type Integer) (bFromSweep :type Boolean) (SweepResult :type "HitResult Structure (by ref)"))
  (if (`KismetSystemLibrary.DoesImplementInterface` OtherActor "/Game/BP/Player/BPI_Player.BPI_Player_C")
    (`SceneComponent.SetHiddenInGame` (`self.FloorSprite`) true false)
    (`ActorComponent.SetActive` (`self.Sphere`) false false)
    (message `/Game/BP/Player/BPI_Player.AddToInventory` OtherActor (make `/Game/BP/Weapons/WeaponData` (`self.ManualWeapon`) (`self.DistanceAttack`) (`self.weaponDamage`) (`self.Weapon Sprite`) (`self.Weapon Idle Anim`) (`self.Weapon Shoot Anim`)))
    (`self.K2_DestroyActor`)))

(event `/Game/BP/Weapons/BPI_Weapon.ShootLoop`
  (bind _weaponflipbook (`self.WeaponFlipbook`))
  (if (not (`self.ManualWeapon`))
    (`PaperFlipbookComponent.SetLooping` (`self.WeaponFlipbook`) true)
    (`self.FireWeapon` :!label _label)
    (`PaperFlipbookComponent.SetFlipbook` _weaponflipbook (`self.Weapon Shoot Anim`))
    (if (`self.ManualWeapon`)
      (`KismetSystemLibrary.Delay` (`PaperFlipbookComponent.GetFlipbookLength` _weaponflipbook))
      (`PaperFlipbookComponent.SetFlipbook` _weaponflipbook (`self.Weapon Idle Anim`))
      (`self.ResetWeapon`))))

(event `/Game/BP/Weapons/BPI_Weapon.Shoot`
  (if (`self.ManualWeapon`)
    (`/Engine/EditorBlueprintResources/StandardMacros.DoOnce` false :!label _label_2
      (:`Completed`
        (goto _label)))))

(event `ResetWeapon`
  (goto _label_2 :!via `Reset`))

(event `/Game/BP/Weapons/BPI_Weapon.CancelShoot`
  (if (not (`self.ManualWeapon`))
    (`PaperFlipbookComponent.SetFlipbook` (`self.WeaponFlipbook`) (`self.Weapon Idle Anim`))))

(event `/Game/BP/Weapons/BPI_Weapon.SetData`
  (params (data :type "/Game/BP/Weapons/WeaponData Structure"))
  (set `self.IsPunch` data_isPunch_19_AEC643BB4ED50919F9569EB89D407963)
  (set `self.ManualWeapon` data_Manual_1_1918408D4FFFB21AD6B155B37DB56483)
  (set `self.DistanceAttack` data_DistanceAttack_5_5525C8444713E52E3BE335BCDD5CF29B)
  (set `self.weaponDamage` data_Damage_7_8990B3394EE8884388BF4994D92E3D07)
  (set `self.Weapon Sprite` data_WeaponSprite_16_47327AB941EE913525F28FBD2C75E547)
  (bind _output_get (set `self.Weapon Idle Anim` data_WeaponIdleAnim_14_4232EA10485305FD8950809CAC94EC03))
  (set `self.Weapon Shoot Anim` data_WeaponShootAnim_15_3186D38542403C5A5CF14DB0B7B10870)
  (`PaperFlipbookComponent.SetFlipbook` (`self.WeaponFlipbook`) _output_get))

(fn `FireWeapon`
  (locals (WorldLocation :type "Vector Structure") (ForwardVector :type "Vector Structure"))
  (bind _defaultsceneroot (`self.DefaultSceneRoot`))
  (bind _weapondamage (`self.weaponDamage`))
  (bind _returnvalue (`SceneComponent.K2_GetComponentLocation` _defaultsceneroot))
  (bind (_returnvalue_x _returnvalue_y) (`KismetMathLibrary.BreakVector` (`SceneComponent.GetForwardVector` _defaultsceneroot)))
  (bind _returnvalue_2 (`KismetMathLibrary.MakeVector` _returnvalue_x _returnvalue_y))
  (set `self.HitActor` (`self.ResetActor`))
  (for _index (range -10 16)
    (bind _returnvalue_3 (* _index 10))
    (bind _outhit (`KismetSystemLibrary.LineTraceSingle` (+ (+ _returnvalue _returnvalue_2) (`KismetMathLibrary.MakeVector` 0.0 0.0 _returnvalue_3)) (+ (+ _returnvalue (* _returnvalue_2 (`self.DistanceAttack`))) (`KismetMathLibrary.MakeVector` 0.0 0.0 _returnvalue_3)) "TraceTypeQuery3"))
    (bind (_bblockinghit _binitialoverlap _time _distance _location _impactpoint _normal _impactnormal _physmat _hitactor) (`GameplayStatics.BreakHitResult` _outhit))
    (if (`KismetSystemLibrary.DoesImplementInterface` _hitactor "/Game/BP/Ennemie/BPI_Ennemie.BPI_Ennemie_C")
      (message `/Game/BP/Player/BPI_Player.ApplyHit` (`GameplayStatics.GetPlayerCharacter` 0) _hitactor (`KismetMathLibrary.SelectFloat` _weapondamage (/ _weapondamage (`self.Delta Seconds`)) (`self.ManualWeapon`)))
      (break)
      (else
        (`/Engine/EditorBlueprintResources/StandardMacros.IsValid` _hitactor
          (:`Is Valid`
            (bind _returnvalue_4 (`KismetMathLibrary.Vector_Distance` (`self.K2_GetActorLocation` _hitactor) (`self.K2_GetActorLocation` (`GameplayStatics.GetPlayerCharacter` 0))))
            (if (and (`self.IsPunch`) (and (<= _returnvalue_4 130.0) (>= _returnvalue_4 80.0)))
              (message `/Game/BP/Player/BPI_Player.ParryBulletPlayer` (`GameplayStatics.GetPlayerCharacter` 0) _hitactor (`self.GetActorForwardVector`))
              (break))))))))

(fn `UserConstructionScript`)